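; Openable door actor that swings open and shut when its OpenDoor component fires open and close events.
; The OpenDoor component's code triggers the DoorSwing timeline, playing it forward to open and reversing it to close.
; The timeline's yaw angle is combined with the rotation saved at BeginPlay, so doors open relative to their placement.
; A Sound Timing event track on the timeline plays a door lock sound at the actor's location.
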(event OnOpen(OpenDoor)
  ;[1 1 1] These come from code off the OpenDoor Component
  (bind _openangle (Timeline|DoorSwing Play)
    (:Update
      (Transformation|SetActorRotation (Math|Rotator|CombineRotators (Math|Rotator|MakeRotator 0.0 0.0 _openangle) (Variables|Default|GetInitialRotation))))
    (:SoundTiming
      (Audio|PlaySoundatLocation "/Game/door-lock.door-lock" (Transformation|GetActorLocation)))))

(event OnClose(OpenDoor)
  ;[1 1 1] These come from code off the OpenDoor Component
  (bind _openangle (Timeline|DoorSwing Reverse)
    (:Update
      (Transformation|SetActorRotation (Math|Rotator|CombineRotators (Math|Rotator|MakeRotator 0.0 0.0 _openangle) (Variables|Default|GetInitialRotation))))
    (:SoundTiming
      (Audio|PlaySoundatLocation "/Game/door-lock.door-lock" (Transformation|GetActorLocation)))))

(event EventBeginPlay
  (Variables|Default|SetInitialRotation (Transformation|GetActorRotation)))

(fn ConstructionScript)